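; Machine gun weapon Blueprint that spawns projectiles from its GunPoint component while the Shoot input is held.
; It enables input for player 0 on BeginPlay.
; Pressing and releasing Shoot toggles IsShooting and mirrors it to IsShootingAnim on the mesh's ABP_MachineGun anim instance.
; While shooting, Tick feeds a short Delay that paces the fire rate, spawning each projectile at GunPoint's location and rotation.
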(event `self.ReceiveBeginPlay`
  ;[1 1 1] Enable input for weapon
  (`self.EnableInput` (`GameplayStatics.GetPlayerController` 0)))

(event `InputAction|Shoot`
  (params (Key :type "Key Structure" :default "AnyKey"))
  (bind _returnvalue (`SkeletalMeshComponent.GetAnimInstance` (`self.SK_MachineGunn`)))
  ;[1 1 1] Weapon Input
  (:`Pressed`
    (set `self.isShooting` true)
    (bind _asabp_machine_gun (cast `/Game/Scripting/Animation_Blueprints/ABP_MachineGun` _returnvalue))
    (set `/Game/Scripting/Animation_Blueprints/ABP_MachineGun.isShootingAnim` true _asabp_machine_gun))
  (:`Released`
    (set `self.isShooting` false)
    (bind _asabp_machine_gun_2 (cast `/Game/Scripting/Animation_Blueprints/ABP_MachineGun` _returnvalue))
    (set `/Game/Scripting/Animation_Blueprints/ABP_MachineGun.isShootingAnim` false _asabp_machine_gun_2)))

(event `self.ReceiveTick`
  (params (DeltaSeconds :type "Float (single-precision)"))
  ;[1 1 1] Spawn projeciles when isShooting is true
  (if (`self.isShooting`)
    (`KismetSystemLibrary.Delay` 0.1)
    (`|SpawnActorFromClass` "/Game/Scripting/Projectiles/Projectile.Projectile_C" (`KismetMathLibrary.MakeTransform` (`SceneComponent.K2_GetComponentLocation` (`self.GunPoint`)) (`SceneComponent.K2_GetComponentRotation` (`self.GunPoint`))) "Undefined" "OverrideRootScale")))

(fn `UserConstructionScript`)